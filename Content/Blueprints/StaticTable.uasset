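; StaticTable is an actor that holds a reference to the level's Database actor and, as wired, stays where it is placed.
; BeginPlay finds all Database actors and caches the first as DatabaseActor.
; A disconnected SetActorLocation would lower it along Z by the Database's Velocity scaled by delta time, but Tick is empty, so that movement never runs.
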(event `self.ReceiveBeginPlay`
  (bind _outactors (`GameplayStatics.GetAllActorsOfClass` "/Game/Blueprints/Database.Database_C"))
  (set `self.DatabaseActor` (`|GetArrayItem` _outactors)))

(event `self.ReceiveTick`
  (params (DeltaSeconds :type "Float (single-precision)")))

(fn `UserConstructionScript`)