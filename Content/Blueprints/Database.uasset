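; Database is a Blueprint that drives a growing speed value and a score derived from it.
; On BeginPlay a looping one-second timer calls Increase Velocity.
; Each call compounds Velocity by two percent and, while it is nonzero, sets Score to the truncated amount above a base of one hundred.
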(event `self.ReceiveBeginPlay`
  (`KismetSystemLibrary.K2_SetTimer` null "Increase Velocity" 1.0 true))

(fn `Increase Velocity`
  (bind _velocity (`self.Velocity`))
  (bind _output_get (set `self.Velocity` (+ _velocity (* _velocity 0.02))))
  (if (not (== _output_get 0.0))
    (set `self.Score` (`KismetMathLibrary.FTrunc` (- _output_get 100.0)))))

(fn `UserConstructionScript`)