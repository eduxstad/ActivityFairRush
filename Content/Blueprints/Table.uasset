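; Table is an obstacle actor that moves downward and ends the game when its box overlaps the 2D side-scroller character.
; On spawn it occasionally shows a random decoration, either one of three sprites or a club name drawn from a list.
; Each tick it descends at the velocity held by a shared Database actor.
; On player contact it zeroes that velocity, sets the pause flag and replaces all widgets with GameOverUI.
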(event `self.ReceiveBeginPlay`
  (bind _outactors (`GameplayStatics.GetAllActorsOfClass` "/Game/Blueprints/Database.Database_C"))
  (set `self.DatabaseActor` (`|GetArrayItem` _outactors))
  (if (== (`KismetMathLibrary.RandomInteger` 5) 4)
    (if (`KismetMathLibrary.RandomBool`)
      (if (`KismetMathLibrary.RandomBool`)
        (`SceneComponent.SetVisibility` (`self.svg-sprite-chess-piece-3_Sprite`) true false)
        (elif (`KismetMathLibrary.RandomBool`)
          (`SceneComponent.SetVisibility` (`self.flag_Sprite`) true false)
          (else
            (`SceneComponent.SetVisibility` (`self.index_Sprite`) true false))))
      (else
        (`TextRenderComponent.K2_SetText` (`self.TextRender`) (`|GetArrayItem` (`self.Clubs`) (`KismetMathLibrary.RandomInteger` (`KismetArrayLibrary.Array_Length` (`self.Clubs`)))))))))

(event `self.ReceiveActorBeginOverlap`
  (params (OtherActor :type "Actor Object Reference")))

(event `self.ReceiveTick`
  (params (DeltaSeconds :type "Float (single-precision)"))
  (`self.K2_SetActorLocation` (`KismetMathLibrary.MakeVector` (.x (`self.K2_GetActorLocation`)) (.y (`self.K2_GetActorLocation`)) (- (.z (`self.K2_GetActorLocation`)) (* DeltaSeconds (`/Game/Blueprints/Database.Velocity` (`self.DatabaseActor`)))))))

(event `self.Box.OnComponentBeginOverlap`
  (params (OverlappedComponent :type "PrimitiveComponent Object Reference") (OtherActor :type "Actor Object Reference") (OtherComp :type "PrimitiveComponent Object Reference") (OtherBodyIndex :type Integer) (bFromSweep :type Boolean) (SweepResult :type "HitResult Structure (by ref)"))
  (bind _databaseactor (`self.DatabaseActor`))
  (if (`KismetStringLibrary.EqualEqual_StrStr` (`KismetSystemLibrary.GetDisplayName` OtherActor) "2DSideScrollerCharacter")
    (set `/Game/Blueprints/Database.Velocity` 0.0 _databaseactor)
    (set `/Game/Blueprints/Database.GamePause` true _databaseactor)
    (`WidgetLayoutLibrary.RemoveAllWidgets`)
    (bind _returnvalue (`|CreateWidget` "/Game/Blueprints/GameOverUI.GameOverUI_C"))
    (bind _output_get (set `self.GameOverUI` _returnvalue))
    (`UserWidget.AddToViewport` _output_get 0)))

(fn `UserConstructionScript`)